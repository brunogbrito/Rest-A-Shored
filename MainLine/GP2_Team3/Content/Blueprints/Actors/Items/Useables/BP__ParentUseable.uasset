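; Base Blueprint for useable world items that BP_CoolDude can pick up, drop and eat, with a name-label widget.
; Mesh overlaps register it as a visible interactable on TTCharacters and toggle the label.
; Pickup and drop montage notifies drive hand-socket attachment or detachment, with sounds and random speech balloons, while physics toggles.
; Use passes the item name to the character's CustomEat; being eaten destroys the actor.
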(event OnDrop(TTEquipable)
  (params (equiper :type TT%20Equiper%20Component%20Object%20Reference))
  ;[1 1 1] Drop
  (bind _asbp_cool_dude (Utilities|Casting|CastToBP_CoolDude (Components|GetOwner equiper)))
  (Animation|Montage|PlayMontage (Variables|/Script/Engine.Character|GetMesh _asbp_cool_dude) "/Game/3D/Animation/Human/AM_Drop.AM_Drop"
    (:OnNotifyBegin
      (Transformation|DetachFromActor "KeepWorld" "KeepWorld" "KeepWorld")
      (Rendering|SetVisibility (Variables|Default|GetWidget) true false)
      (Physics|SetSimulatePhysics (Variables|Default|GetStaticMesh) true)
      ;;[1 0 0.6595] Comment
      (bind _ondrop (Variables|Default|GetOnDrop)
        (:then
          (Audio|PlaySound2D _ondrop 1.0 1.0 0.0 0 0)
          ;;[0.1683 1 0] Comment
          (bind (_output _returnvalue) (CallFunction|GetRandomTextMessagefromArray (Variables|Default|GetOnDroped)))
          (Default|PopUPBaloon _asbp_cool_dude _output 2.5 _returnvalue))
        (:else)))))

(event BeenEaten(TTEdible)
  ;[1 1 1] Drop
  ;;[1 0 0.5985] Comment
  (bind _beingeatenn (Variables|Default|GetBeingEatenn)
    (:then
      (Audio|PlaySound2D _beingeatenn 1.0 1.0 0.0 0 0))
    (:else
      _))
  (Actor|DestroyActor))

(event OnComponentBeginOverlap(StaticMesh)
  (params (OverlappedComponent :type Primitive%20Component%20Object%20Reference) (OtherActor :type Actor%20Object%20Reference) (OtherComp :type Primitive%20Component%20Object%20Reference) (OtherBodyIndex :type Integer) (bFromSweep :type Boolean) (SweepResult :type Hit%20Result%20Structure%20%28by%20ref%29))
  (bind _asttcharacter (Utilities|Casting|CastToTTCharacter OtherActor))
  (Class|TTCharacter|AddVisibleInteractable _asttcharacter (Variables|Default|GetTTInteractable))
  (Rendering|SetVisibility (Variables|Default|GetWidget) true false)
  ;[1 0 0.7046] Comment
  (Audio|PlaySound2D "/Game/Audio/PlaceHolders/InteractablesOn_v01_Cue.InteractablesOn_v01_Cue" 1.0 1.0 0.0 0 0))

(event OnComponentEndOverlap(StaticMesh)
  (params (OverlappedComponent :type Primitive%20Component%20Object%20Reference) (OtherActor :type Actor%20Object%20Reference) (OtherComp :type Primitive%20Component%20Object%20Reference) (OtherBodyIndex :type Integer))
  (bind _asttcharacter (Utilities|Casting|CastToTTCharacter OtherActor))
  (Class|TTCharacter|RemoveVisibleInteractable _asttcharacter (Variables|Default|GetTTInteractable))
  (Rendering|SetVisibility (Variables|Default|GetWidget) false false)
  ;[1 0 0.7046] Comment
  (Audio|PlaySound2D "/Game/Audio/PlaceHolders/InteractablesOn_v01_Cue.InteractablesOn_v01_Cue" 1.0 1.0 0.0 0 0))

(event OnPickup(TTEquipable)
  (params (equiper :type TT%20Equiper%20Component%20Object%20Reference))
  (bind _staticmesh (Variables|Default|GetStaticMesh))
  ;[1 1 1] Pick Up
  (bind _asbp_cool_dude (Utilities|Casting|CastToBP_CoolDude (Components|GetOwner equiper)))
  (Animation|Montage|PlayMontage (Variables|/Script/Engine.Character|GetMesh _asbp_cool_dude) "/Game/3D/Animation/Human/AM_PickUp.AM_PickUp"
    (:then
      (Physics|SetSimulatePhysics _staticmesh false)
      (Transformation|ResetRelativeTransform _staticmesh))
    (:OnNotifyBegin
      (Transformation|AttachComponentToComponent (Variables|/Script/Engine.Character|GetMesh _asbp_cool_dude) "RightHandSocket" "SnapToTarget" "SnapToTarget" "KeepWorld" true)
      ;;[1 0 0.6595] Comment
      (bind _onpickup (Variables|Default|GetOnPickUp)
        (:then
          (Audio|PlaySound2D _onpickup 1.0 1.0 0.0 0 0))
        (:else
          _))
      ;;[0.1683 1 0] Comment
      (bind (_output _returnvalue) (CallFunction|GetRandomTextMessagefromArray (Variables|Default|GetOnPicked)))
      (Default|PopUPBaloon _asbp_cool_dude _output 2.5 _returnvalue)
      (bind _asttcharacter (Utilities|Casting|CastToTTCharacter (stale OnComponentEndOverlap(StaticMesh) OtherActor)))
      (Class|TTCharacter|RemoveVisibleInteractable _asttcharacter (Variables|Default|GetTTInteractable))
      (Rendering|SetVisibility (Variables|Default|GetWidget) false false)
      ;[1 0 0.7046] Comment
      (Audio|PlaySound2D "/Game/Audio/PlaceHolders/InteractablesOn_v01_Cue.InteractablesOn_v01_Cue" 1.0 1.0 0.0 0 0))))

(event OnPickup(TTInteractable)
  (params (interactor :type TT%20Interactor%20Component%20Object%20Reference) (inventory :type TT%20Inventory%20Component%20Object%20Reference))
  (Rendering|SetVisibility (Variables|Default|GetWidget) false false))

(event OnDrop(TTInteractable)
  (params (interactor :type TT%20Interactor%20Component%20Object%20Reference))
  (Rendering|SetVisibility (Variables|Default|GetWidget) true false))

(event OnUse(TTInteractable)
  (params (equiper :type TT%20Equiper%20Component%20Object%20Reference) (equipment :type Actor%20Object%20Reference))
  (bind _asbp_cool_dude (Utilities|Casting|CastToBP_CoolDude (Components|GetOwner equiper)))
  (Default|CustomEat _asbp_cool_dude (Utilities|String|ToString(Name) (Variables|Default|GetName))))

(event EventBeginPlay
  (bind _returnvalue (UserInterface|CreateWidget "/Game/Blueprints/UI/WBP_Items.WBP_Items_C" (Game|GetPlayerController 0)))
  (Variables|/Game/Blueprints/UI/WBP_Items.WBP_Items_C|SetItemText _returnvalue (Utilities|Text|ToText(Name) (Variables|Default|GetName)))
  (UserInterface|SetWidget (Variables|Default|GetWidget) _returnvalue))

(fn ConstructionScript)