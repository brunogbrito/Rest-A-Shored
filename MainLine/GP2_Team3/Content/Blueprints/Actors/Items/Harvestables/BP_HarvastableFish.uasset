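; Harvestable fish actor that players gather with a specific equipment class, yielding resources to the user's inventory component.
; Using it advances harvest progression and calls GetResource, while any other valid equipment stops the interaction.
; On depletion the mesh hides and loses collision, then returns after a respawn delay.
; A sphere overlap registers the interactable with TTCharacter, toggles the prompt widget and plays a cue.
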(event OnComponentBeginOverlap(Sphere)
  (params (OverlappedComponent :type Primitive%20Component%20Object%20Reference) (OtherActor :type Actor%20Object%20Reference) (OtherComp :type Primitive%20Component%20Object%20Reference) (OtherBodyIndex :type Integer) (bFromSweep :type Boolean) (SweepResult :type Hit%20Result%20Structure%20%28by%20ref%29))
  (bind _asttcharacter (Utilities|Casting|CastToTTCharacter OtherActor))
  (Class|TTCharacter|AddVisibleInteractable _asttcharacter (Variables|Default|GetTTInteractable))
  (Rendering|SetVisibility (Variables|Default|GetWidget) true false)
  (Audio|PlaySound2D "/Game/Audio/PlaceHolders/InteractablesOn_v01_Cue.InteractablesOn_v01_Cue" 1.0 1.0 0.0 0 0))

(event OnComponentEndOverlap(Sphere)
  (params (OverlappedComponent :type Primitive%20Component%20Object%20Reference) (OtherActor :type Actor%20Object%20Reference) (OtherComp :type Primitive%20Component%20Object%20Reference) (OtherBodyIndex :type Integer))
  (bind _asttcharacter (Utilities|Casting|CastToTTCharacter OtherActor))
  (Class|TTCharacter|RemoveVisibleInteractable _asttcharacter (Variables|Default|GetTTInteractable))
  (Rendering|SetVisibility (Variables|Default|GetWidget) false false)
  (Audio|PlaySound2D "/Game/Audio/PlaceHolders/InteractablesOn_v01_Cue.InteractablesOn_v01_Cue" 1.0 1.0 0.0 0 0))

(event EventBeginPlay
  (|CallParentFunction))

(event Collision|EventActorBeginOverlap
  (params (OtherActor :type Actor%20Object%20Reference))
  (|CallParentFunction OtherActor) ; This node is disabled and will not be called.\nDrag off pins to build functionality.
)

(event EventOnHarvested)

(event EventOnUse
  (params (Equiper :type TT%20Equiper%20Component%20Object%20Reference) (Equipment :type Actor%20Object%20Reference) (DeltaTime :type Float%20%28single-precision%29))
  (Utilities|IsValid Equipment
    (:Is%20Valid
      (if (== (Utilities|GetClass Equipment) (Variables|Default|GetActorReference))
        (Class|TTHarvestable|UpdateProgression (Variables|Default|GetTTHarvestable) DeltaTime)
        (CallFunction|GetResource (Transformation|GetActorTransform) (Actor|GetComponentbyClass (Components|GetOwner Equiper) "/Script/GP2_Team3.TTInventoryComponent"))
        (else
          (Class|TTInteractableComponent|StopInteraction (Variables|Default|GetTTInteractable)))))))

(event EventOnResourceDepleted
  (|CallParentFunction)
  (Rendering|SetVisibility (Variables|Default|GetStaticMesh) false false)
  (Collision|SetCollisionEnabled (Variables|Default|GetStaticMesh) "NoCollision")
  (Utilities|FlowControl|Delay (Variables|Default|GetTimerRespawnFish))
  (Rendering|SetVisibility (Variables|Default|GetStaticMesh) true false)
  (Collision|SetCollisionEnabled (Variables|Default|GetStaticMesh) "QueryAndPhysics"))

(event EventTick
  (params (DeltaSeconds :type Float%20%28single-precision%29))
  (|CallParentFunction DeltaSeconds) ; This node is disabled and will not be called.\nDrag off pins to build functionality.
)

(fn ConstructionScript
  (|CallParentFunction))