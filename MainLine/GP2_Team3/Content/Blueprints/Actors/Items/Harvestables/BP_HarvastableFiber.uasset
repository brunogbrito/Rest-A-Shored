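; Harvestable fiber resource that characters gather by hand and that respawns after being depleted.
; Use advances the harvest over time and passes the user's inventory to GetResource, but stops the interaction if equipment is held.
; Depletion hides the visuals and disables collision until a respawn delay restores both.
; Sphere overlaps register the interactable with the character, toggle the prompt widget and play a sound.
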(event OnComponentBeginOverlap(Sphere)
  (params (OverlappedComponent :type Primitive%20Component%20Object%20Reference) (OtherActor :type Actor%20Object%20Reference) (OtherComp :type Primitive%20Component%20Object%20Reference) (OtherBodyIndex :type Integer) (bFromSweep :type Boolean) (SweepResult :type Hit%20Result%20Structure%20%28by%20ref%29))
  (bind _asttcharacter (Utilities|Casting|CastToTTCharacter OtherActor))
  (Class|TTCharacter|AddVisibleInteractable _asttcharacter (Variables|Default|GetTTInteractable))
  (Rendering|SetVisibility (Variables|Default|GetWidget) true false)
  (Audio|PlaySound2D "/Game/Audio/PlaceHolders/InteractablesOn_v01_Cue.InteractablesOn_v01_Cue" 1.0 1.0 0.0 0 0))

(event OnComponentEndOverlap(Sphere)
  (params (OverlappedComponent :type Primitive%20Component%20Object%20Reference) (OtherActor :type Actor%20Object%20Reference) (OtherComp :type Primitive%20Component%20Object%20Reference) (OtherBodyIndex :type Integer))
  (bind _asttcharacter (Utilities|Casting|CastToTTCharacter OtherActor))
  (Class|TTCharacter|RemoveVisibleInteractable _asttcharacter (Variables|Default|GetTTInteractable))
  (Rendering|SetVisibility (Variables|Default|GetWidget) false false)
  (Audio|PlaySound2D "/Game/Audio/PlaceHolders/InteractablesOn_v01_Cue.InteractablesOn_v01_Cue" 1.0 1.0 0.0 0 0))

(event EventOnResourceDepleted
  (|CallParentFunction)
  (for _array_element (Variables|Default|GetClassContentArray)
    (Rendering|SetVisibility _array_element false true))
  (Collision|SetCollisionEnabled (Variables|Default|GetSphere) "NoCollision")
  (Utilities|FlowControl|Delay (Variables|Default|GetTimerRespawnFiber))
  (for _array_element_2 (Variables|Default|GetClassContentArray)
    (Rendering|SetVisibility _array_element_2 true true))
  (Collision|SetCollisionEnabled (Variables|Default|GetSphere) "QueryAndPhysics"))

(event EventOnUse
  (params (Equiper :type TT%20Equiper%20Component%20Object%20Reference) (Equipment :type Actor%20Object%20Reference) (DeltaTime :type Float%20%28single-precision%29))
  (Utilities|IsValid Equipment
    (:Is%20Valid
      (Class|TTInteractableComponent|StopInteraction (Variables|Default|GetTTInteractable)))
    (:Is%20Not%20Valid
      (Class|TTHarvestable|UpdateProgression (Variables|Default|GetTTHarvestable) DeltaTime)
      (CallFunction|GetResource (Transformation|GetActorTransform) (Actor|GetComponentbyClass (Components|GetOwner Equiper) "/Script/GP2_Team3.TTInventoryComponent")))))

(fn ConstructionScript
  (|CallParentFunction))