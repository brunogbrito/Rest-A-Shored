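; Harvestable water pump item that yields a resource to the actor using it.
; On use, it advances the TTHarvestable progression by delta time, then calls GetResource with a spawn transform offset from the pump and the user's TTInventoryComponent.
; When the resource is depleted, it runs the parent handling and keeps or makes its Widget visible.
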(event EventOnResourceDepleted
  (|CallParentFunction)
  (Rendering|SetVisibility (Variables|Default|GetWidget) true false))

(event EventOnUse
  (params (Equiper :type TT%20Equiper%20Component%20Object%20Reference) (Equipment :type Actor%20Object%20Reference) (DeltaTime :type Float%20%28single-precision%29))
  (bind _returnvalue (Transformation|GetActorTransform))
  (Class|TTHarvestable|UpdateProgression (Variables|Default|GetTTHarvestable) DeltaTime)
  (CallFunction|GetResource (Math|Transform|MakeTransform (+ (.location _returnvalue) "50.000000, 0,150.000000") (.rotation _returnvalue) (.scale _returnvalue)) (Actor|GetComponentbyClass (Components|GetOwner Equiper) "/Script/GP2_Team3.TTInventoryComponent")))

(fn ConstructionScript
  (|CallParentFunction))