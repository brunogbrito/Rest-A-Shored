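; Harvestable tree that characters chop with the required tool to gain resources into their inventory.
; Use advances TTHarvestable progress and grants resources if the equipment class matches; otherwise interaction stops and BP_CoolDude shows a random "need axe" balloon.
; On depletion it removes interaction as a temporary guard on the stump, enables physics on one mesh, then destroys two meshes after a delay.
; RespawnStuff replaces the actor with a fresh copy.
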(event EventOnResourceDepleted
  (bind _staticmesh1 (Variables|Default|GetStaticMesh1))
  (|CallParentFunction)
  (Physics|SetSimulatePhysics _staticmesh1 true)
  (Components|DestroyComponent (Variables|Default|GetTTInteractable)) ; Temp!! To prohibit the characters to interact with the stump
  (Utilities|FlowControl|Delay 5.0)
  (Components|DestroyComponent _staticmesh1))

(event EventOnUse
  (params (Equiper :type TT%20Equiper%20Component%20Object%20Reference) (Equipment :type Actor%20Object%20Reference) (DeltaTime :type Float%20%28single-precision%29))
  (Utilities|IsValid Equipment
    (:Is%20Valid
      (if (== (Utilities|GetClass Equipment) (Variables|Default|GetActorReference))
        (Class|TTHarvestable|UpdateProgression (Variables|Default|GetTTHarvestable) DeltaTime)
        (CallFunction|GetResource (Transformation|GetActorTransform) (Actor|GetComponentbyClass (Components|GetOwner Equiper) "/Script/GP2_Team3.TTInventoryComponent"))
        (else
          (Class|TTInteractableComponent|StopInteraction (Variables|Default|GetTTInteractable) :!label _label)
          ;[0.2166 1 0] Comment
          (bind _asbp_cool_dude (Utilities|Casting|CastToBP_CoolDude (Components|GetOwner Equiper)))
          (bind (_output _returnvalue) (CallFunction|GetRandomTextMessagefromArray (Variables|Default|GetNeedAxe)))
          (Default|PopUPBaloon _asbp_cool_dude _output 2.5 _returnvalue))))
    (:Is%20Not%20Valid
      (goto _label))))

(event EventOnHarvested)

(event EventRespawnStuff
  (Game|SpawnActorfromClass "BP_HarvestbleTree_C" (Transformation|GetActorTransform) "Undefined" 0 0)
  (Utilities|FlowControl|Delay 0.1)
  (Actor|DestroyActor))

(fn ConstructionScript
  (|CallParentFunction))