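; Repairable boat actor that ends the game in victory once its build progress reaches ReadyIndex.
; Overlapping characters register it as a visible interactable, toggling its label widget and the player controller's Repair command with a sound.
; StartBuildingBoat runs a looping one-second timer that increments and displays progress until stopped, triggering GameMode Victory once at the threshold.
; ReadyToBuild sets IsBoatRepairable, but the check on that flag is unconnected.
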(event OnComponentBeginOverlap(StaticMesh)
  (params (OverlappedComponent :type Primitive%20Component%20Object%20Reference) (OtherActor :type Actor%20Object%20Reference) (OtherComp :type Primitive%20Component%20Object%20Reference) (OtherBodyIndex :type Integer) (bFromSweep :type Boolean) (SweepResult :type Hit%20Result%20Structure%20%28by%20ref%29))
  (bind _asttcharacter (Utilities|Casting|CastToTTCharacter OtherActor))
  (Class|TTCharacter|AddVisibleInteractable _asttcharacter (Variables|Default|GetTTInteractable))
  (Rendering|SetVisibility (Variables|Default|GetWidget) true false)
  ;[1 0 0.7046] Comment
  (Audio|PlaySound2D "/Game/Audio/PlaceHolders/InteractablesOn_v01_Cue.InteractablesOn_v01_Cue" 1.0 1.0 0.0 0 0)
  (bind _asbp_player_controller (Utilities|Casting|CastToBP_PlayerController (Game|GetPlayerController 0)))
  (Default|AddActionCommand _asbp_player_controller "Repair"))

(event OnComponentEndOverlap(StaticMesh)
  (params (OverlappedComponent :type Primitive%20Component%20Object%20Reference) (OtherActor :type Actor%20Object%20Reference) (OtherComp :type Primitive%20Component%20Object%20Reference) (OtherBodyIndex :type Integer))
  (bind _asttcharacter (Utilities|Casting|CastToTTCharacter OtherActor))
  (Class|TTCharacter|RemoveVisibleInteractable _asttcharacter (Variables|Default|GetTTInteractable))
  (Rendering|SetVisibility (Variables|Default|GetWidget) false false)
  ;[1 0 0.7046] Comment
  (Audio|PlaySound2D "/Game/Audio/PlaceHolders/InteractablesOn_v01_Cue.InteractablesOn_v01_Cue" 1.0 1.0 0.0 0 0)
  (bind _asbp_player_controller (Utilities|Casting|CastToBP_PlayerController (Game|GetPlayerController 0)))
  (Default|RemoveActionCommand _asbp_player_controller "Repair"))

(event OnStop(TTInteractable)
  (Utilities|Time|ClearandInvalidateTimerbyHandle (Variables|Default|GetTimeHandler)))

(event Custom|StartBuildingBoat
  (bind _returnvalue (Utilities|Time|SetTimerbyEvent (delegate Custom|CustomEvent_0) 1.0 true))
  (Variables|Default|SetTimeHandler _returnvalue))

(event Custom|CustomEvent_0
  (bind _output_get (Variables|Default|SetBoatIndex (+ (Variables|Default|GetBoatIndex) 1)))
  (Variables|/Game/Blueprints/UI/WBP_Items.WBP_Items_C|SetItemText (Variables|Default|GetWBP) (Utilities|Text|FormatText "{NAME} {%}%" (Utilities|Text|ToText(Name) (Variables|Default|GetName)) _output_get))
  (if (>= _output_get (Variables|Default|GetReadyIndex))
    (Development|PrintString (Utilities|String|ToString(Integer) _output_get))
    (Utilities|FlowControl|DoOnce false
      (:Completed
        (bind _asbp_game_mode (Utilities|Casting|CastToBP_GameMode (Game|GetGameMode)))
        (Default|Victory _asbp_game_mode)))))

(event Custom|ReadyToBuild
  (Variables|Default|SetIsBoatRepairable? true))

(event Custom|STOOOP
  (Utilities|Time|ClearandInvalidateTimerbyHandle (Variables|Default|GetTimeHandler)))

(event EventBeginPlay
  (bind _returnvalue (UserInterface|CreateWidget "/Game/Blueprints/UI/WBP_Items.WBP_Items_C" (Game|GetPlayerController 0)))
  (bind _output_get (Variables|Default|SetWBP _returnvalue))
  (Variables|/Game/Blueprints/UI/WBP_Items.WBP_Items_C|SetItemText _output_get (Utilities|Text|ToText(Name) (Variables|Default|GetName)))
  (UserInterface|SetWidget (Variables|Default|GetWidget) _output_get))

(event Collision|EventActorBeginOverlap
  (params (OtherActor :type Actor%20Object%20Reference)))

(event EventTick
  (params (DeltaSeconds :type Float%20%28single-precision%29)))

(fn ConstructionScript)