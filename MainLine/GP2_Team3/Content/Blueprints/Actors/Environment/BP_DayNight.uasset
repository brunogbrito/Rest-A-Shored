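; Environment actor for the day-night cycle that refreshes the sky and crossfades ambient day and night sounds.
; On begin play it caches BP_GameMode, calls its NewDay and starts both sounds, then updates the SkySphere's sun direction every tick.
; Event handlers forward each new day to the game mode and fade DaySound and NightSound in opposite directions when day or night passes.
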(event EventBeginPlay
  (bind _asbp_game_mode (Utilities|Casting|CastToBP_GameMode (Game|GetGameMode)))
  (bind _output_get (Variables|Default|SetGameMode _asbp_game_mode))
  (Default|NewDay _output_get)
  (Audio|Components|Audio|Play (Variables|Default|GetDaySound) 0.0))

(event EventTick
  (params (DeltaSeconds :type Float%20%28single-precision%29))
  (Default|UpdateSunDirection (Variables|Default|GetSkySphere)))

(event EventOnNightPassed
  (Audio|Components|Audio|FadeIn (Variables|Default|GetNightSound) (Variables|Default|GetSoundFadeTime) 0.4 0.0 :!class /Script/Engine.AudioComponent)
  (Audio|Components|Audio|FadeOut (Variables|Default|GetDaySound) (Variables|Default|GetSoundFadeTime) 0.0 :!class /Script/Engine.AudioComponent))

(event EventOnNewDay
  (Default|NewDay (Variables|Default|GetGameMode)))

(event EventOnDayPassed
  (Audio|Components|Audio|FadeIn (Variables|Default|GetDaySound) (Variables|Default|GetSoundFadeTime) 0.3 0.0 :!class /Script/Engine.AudioComponent)
  (Audio|Components|Audio|FadeOut (Variables|Default|GetNightSound) (Variables|Default|GetSoundFadeTime) 0.0 :!class /Script/Engine.AudioComponent))

(fn ConstructionScript)