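; Game mode that handles the win and lose screens and a random daily weather system.
; BeginPlay caches the temperature handler and command system, and the CharactersAlive OnRep triggers GameOver when none remain.
; NewDay destroys the active weather actor, then randomly picks rain, wind, sun or fog.
; Each weather event spawns its actor at a fixed location, updates the world temperature and NewDay records the weather enum.
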(event Custom|GameOver
  (bind _returnvalue (UserInterface|CreateWidget "/Game/Blueprints/UI/WPB_GameOver.WPB_GameOver_C" (Game|GetPlayerController 0)))
  (UserInterface|Viewport|AddtoViewport _returnvalue 2))

(event Custom|Victory
  (bind _returnvalue (UserInterface|CreateWidget "/Game/Blueprints/UI/WPB_Victory.WPB_Victory_C" (Game|GetPlayerController 0)))
  (UserInterface|Viewport|AddtoViewport _returnvalue 2))

(event Custom|New%20Day
  ;[0 1 0.1948] Weather System
  ;;[1 1 1] Trigger different weathers, random by int
  (bind _activeweather (Variables|Default|GetActiveWeather)
    (:then
      (Actor|DestroyActor _activeweather))
    (:else
      _))
  (switch int (Math|Random|RandomIntegerinRange 0 (- (Variables|Default|GetNumberOfWeathers) 1))
    (:0
      (CallFunction|Rainy)
      (Variables|Default|SetWeatherEnum "NewEnumerator2"))
    (:1
      (CallFunction|Windy)
      (Variables|Default|SetWeatherEnum "NewEnumerator1"))
    (:2
      (CallFunction|Sunny)
      (Variables|Default|SetWeatherEnum "NewEnumerator0"))
    (:3
      (CallFunction|Foggy)
      (Variables|Default|SetWeatherEnum "NewEnumerator3")))
  (Development|PrintString "I am stuff"))

(event Custom|Sunny
  ;[0 1 0.1948] Weather System
  ;;[1 1 1] Spawn Sunny
  (bind _tempraturehandler (Variables|Default|GetTempratureHandler)
    (:then
      (bind _returnvalue (Game|SpawnActorfromClass "/Game/Blueprints/Actors/Environment/BP_ChildSunny.BP_ChildSunny_C" (Math|Transform|MakeTransform "-290.000000,570.000000,1340.000000" "0, 0, 0" "1,1,1") "Undefined" 0 0))
      (Variables|Default|SetActiveWeather _returnvalue)
      ;;;[1 1 1] Set Temprature
      (Class|TTHandlerThermometerComponent|UpdateWorldTemperature _tempraturehandler 8e+01)
      (Development|PrintString "Hello"))
    (:else)))

(event Custom|Rainy
  ;[0 1 0.1948] Weather System
  ;;[1 1 1] Spawn Rain
  (bind _tempraturehandler (Variables|Default|GetTempratureHandler)
    (:then
      (bind _returnvalue (Game|SpawnActorfromClass "/Game/Blueprints/Actors/Environment/BP_ChildRain.BP_ChildRain_C" (Math|Transform|MakeTransform "-9405.000000,-2423.000000,-654.000000" "0,-20.000000, 0" "1,1,1") "Undefined" 0 0))
      (Variables|Default|SetActiveWeather _returnvalue)
      ;;;[1 1 1] Set Temprature
      (Class|TTHandlerThermometerComponent|UpdateWorldTemperature _tempraturehandler 15.0)
      (Development|PrintString "Hello"))
    (:else)))

(event Custom|Foggy
  ;[0 1 0.1948] Weather System
  ;;[1 1 1] Spawn Fog
  (bind _tempraturehandler (Variables|Default|GetTempratureHandler)
    (:then
      (bind _returnvalue (Game|SpawnActorfromClass "/Game/Blueprints/Actors/Environment/BP_ChildFog.BP_ChildFog_C" (Math|Transform|MakeTransform "-1520.000000,1070.000000,-870.000000" "0, 0, 0" "1,1,1") "Undefined" 0 0))
      (Variables|Default|SetActiveWeather _returnvalue)
      ;;;[1 1 1] Set Temprature
      (Class|TTHandlerThermometerComponent|UpdateWorldTemperature _tempraturehandler 4e+01)
      (Development|PrintString "Hello"))
    (:else)))

(event Custom|Windy
  ;[0 1 0.1948] Weather System
  ;;[1 1 1] Spawn Wind
  (bind _tempraturehandler (Variables|Default|GetTempratureHandler)
    (:then
      (bind _returnvalue (Game|SpawnActorfromClass "/Game/Blueprints/Actors/Environment/BP_ChildWindy.BP_ChildWindy_C" (Math|Transform|MakeTransform "-290.000000,570.000000,1340.000000" "0, 0, 0" "1,1,1") "Undefined" 0 0))
      (Variables|Default|SetActiveWeather _returnvalue)
      ;;;[1 1 1] Set Temprature
      (Class|TTHandlerThermometerComponent|UpdateWorldTemperature _tempraturehandler 3e+01)
      (Development|PrintString "Hello"))
    (:else)))

(event EventBeginPlay
  (bind _outactors (Actor|GetAllActorsOfClass "/Script/GP2_Team3.TTHandlerThermometerComponent"))
  (Variables|Default|SetTempratureHandler (Utilities|Array|Get(acopy) _outactors))
  (Variables|Default|SetCharactersAlive (.CharactersAlive (Utilities|GetClassDefaults "BP_GameMode_C")))
  (bind _returnvalue (Class|TTGameMode|GetCommandSystem))
  (Variables|Default|SetCommandSystem _returnvalue))

(fn ConstructionScript)

(fn OnRepCharactersAlive
  (if (<= (Variables|Default|GetCharactersAlive) 0)
    (CallFunction|GameOver)))