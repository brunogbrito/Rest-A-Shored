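; Dog NPC Blueprint that responds to pats and calls through mood and interactable components.
; A BP_CoolDude entering its sphere starts the dog's AI controller and switches the mesh's fade parameter on.
; Pats run a mood check as a Punch social type and adjust mood, with rejection zeroing the effect.
; Accepted calls store the caller and set a Blackboard flag; Tick updates idle time, though boredom has no response.
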(event OnGotBored(TTMood)
  (params (mood :type Integer)))

(event OnGetPated(TTInteractable)
  (params (interactor :type TT%20Interactor%20Component%20Object%20Reference))
  (CallFunction|GetSocilized interactor 0 "Punch"))

(event OnGetCalled(TTInteractable)
  (params (interactor :type TT%20Interactor%20Component%20Object%20Reference))
  (Utilities|GetOwnerComponent interactor "/Script/GP2_Team3.TTMoodComponent"
    (:Is%20Valid
      (bind _returnvalue (Class|TTMoodComponent|DoILikeThis (Variables|Default|GetTTMood) "Call" 0 false))
      (if _returnvalue
        (bind _actor (Utilities|GetInteractor interactor)
          (:Is%20Valid
            (Variables|Default|SetCaller _actor)
            (AI|Components|Blackboard|SetValueasBool (AI|GetBlackboard 0) (Variables|Default|GetCallerName) true)))))))

(event OnComponentBeginOverlap(Sphere)
  (params (OverlappedComponent :type Primitive%20Component%20Object%20Reference) (OtherActor :type Actor%20Object%20Reference) (OtherComp :type Primitive%20Component%20Object%20Reference) (OtherBodyIndex :type Integer) (bFromSweep :type Boolean) (SweepResult :type Hit%20Result%20Structure%20%28by%20ref%29))
  (Utilities|Casting|CastToBP_CoolDude OtherActor)
  (bind _asbp_ai_dog_controller (Utilities|Casting|CastToBP_AI_Dog_controller (Pawn|GetController)))
  (Default|StartAI _asbp_ai_dog_controller)
  (Rendering|Material|SetScalarParameterValueonMaterials (Variables|Character|GetMesh) "Fade ON/OFF" 1.0))

(event EventBeginPlay
  (Rendering|Material|SetScalarParameterValueonMaterials (Variables|Character|GetMesh) "Fade ON/OFF" 0.0))

(event EventTick
  (params (DeltaSeconds :type Float%20%28single-precision%29))
  (Class|TTMoodComponent|TickIdleTime (Variables|Default|GetTTMood) DeltaSeconds))

(fn ConstructionScript)

(fn GetSocilized
  (params (Interactor :type Actor%20Component%20Object%20Reference) (RejectionModifier :type Integer) (socialisingType :type ESocialisingType%20Enum :default "Punch"))
  (bind _output_get (Variables|Default|SetMoodRef (Actor|GetComponentbyClass (Components|GetOwner Interactor) "/Script/GP2_Team3.TTMoodComponent")))
  (Utilities|IsValid _output_get
    (:Is%20Valid
      (bind _returnvalue (Class|TTMoodComponent|DoILikeThis (Variables|Default|GetTTMood) socialisingType (Variables|Default|GetMoodRef) false))
      (if _returnvalue
        (Class|TTMoodComponent|ChangeMoodTowards (Variables|Default|GetMoodRef) (Variables|Default|GetTTMood) (Variables|/Script/GP2_Team3.TTMoodComponent|GethighfiveMoodEffect (Variables|Default|GetMoodRef)))
        (Class|TTMoodComponent|ChangeMyMood (Variables|Default|GetMoodRef) (Variables|/Script/GP2_Team3.TTMoodComponent|GethighfiveMoodEffect (Variables|Default|GetMoodRef)))
        (return true)
        (else
          (Class|TTMoodComponent|ChangeMoodTowards (Variables|Default|GetMoodRef) (Variables|Default|GetTTMood) (* (Variables|/Script/GP2_Team3.TTMoodComponent|GethighfiveMoodEffect (Variables|Default|GetMoodRef)) RejectionModifier))
          (Class|TTMoodComponent|ChangeMyMood (Variables|Default|GetMoodRef) (* (Variables|/Script/GP2_Team3.TTMoodComponent|GethighfiveMoodEffect (Variables|Default|GetMoodRef)) RejectionModifier))
          (return false))))))