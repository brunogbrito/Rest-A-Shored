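; Main menu player controller: Space flushes level streaming and opens the island level, and a separate event shows a loading screen.
; It also holds helpers for speech recognition tuning, caching pawn, game mode and Note actors, and spawning tutorial widgets, none called within its graphs.
; Action command helpers create widgets, track active ones in WidgetArray and redistribute them across three HUD vertical boxes as commands change.
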(event Custom|AddLoadingScreen
  (bind _returnvalue (UserInterface|CreateWidget "/Game/Blueprints/UI/WPB_LoadingGame.WPB_LoadingGame_C" (Game|GetPlayerController 0)))
  (bind _output_get (Variables|Default|SetLoadingScreen _returnvalue))
  (UserInterface|Viewport|AddtoViewport _output_get 2))

(event Input|KeyboardEvents|SpaceBar
  (params (Key :type Key%20Structure))
  (:Pressed
    (Class|GameplayStatics|FlushLevelStreaming)
    (Game|OpenLevel(byName) "Main_IslandPersistent")))

(fn ConstructionScript)

(fn SetConfig
  (bind _speechrecognition (Variables|Default|GetSpeechRecognition))
  (Class|SpeechRecognitionActor|SetConfigParam _speechrecognition "-vad_prespeech" "VE_INTEGER" "10")
  (Class|SpeechRecognitionActor|SetConfigParam _speechrecognition "-vad_postspeech" "VE_INTEGER" "10")
  (Class|SpeechRecognitionActor|SetConfigParam _speechrecognition "-agc" "VE_STRING" "noise")
  (Class|SpeechRecognitionActor|SetConfigParam _speechrecognition "-beam" "VE_FLOAT" "1e-40"))

(fn InitializePlayerController
  (bind _asbp_camera_pawn (Utilities|Casting|CastToBP_CameraPawn (Game|Player|GetPlayerPawn 0)))
  (Variables|Default|SetCameraPawn _asbp_camera_pawn)
  (bind _asbp_game_mode (Utilities|Casting|CastToBP_GameMode (Game|GetGameMode)))
  (bind _output_get (Variables|Default|SetGM _asbp_game_mode))
  (bind _returnvalue (Class|TTGameMode|GetCommandSystem _output_get))
  (bind _outactors (Actor|GetAllActorsOfClass "/Script/Engine.Note"))
  (Variables|Default|SetSpawnLocations _outactors)
  (return _returnvalue))

(fn CreateActionWidgets
  (bind _returnvalue (Game|GetPlayerController 0))
  (bind _returnvalue_2 (UserInterface|CreateWidget "/Game/Blueprints/UI/Actions/WBP_Action_Collect.WBP_Action_Collect_C" _returnvalue))
  (Variables|Default|SetActionCollect _returnvalue_2)
  (bind _returnvalue_3 (UserInterface|CreateWidget "/Game/Blueprints/UI/Actions/WBP_Action_Craft.WBP_Action_Craft_C" _returnvalue))
  (Variables|Default|SetActionCraft _returnvalue_3)
  (bind _returnvalue_4 (UserInterface|CreateWidget "/Game/Blueprints/UI/Actions/WBP_Action_Drop.WBP_Action_Drop_C" _returnvalue))
  (Variables|Default|SetActionDrop _returnvalue_4)
  (bind _returnvalue_5 (UserInterface|CreateWidget "/Game/Blueprints/UI/Actions/WBP_Action_Equip.WBP_Action_Equip_C" _returnvalue))
  (Variables|Default|SetActionEquip _returnvalue_5)
  (bind _returnvalue_6 (UserInterface|CreateWidget "/Game/Blueprints/UI/Actions/WBP_Action_PickUp.WBP_Action_PickUp_C" _returnvalue))
  (Variables|Default|SetActionPickUp _returnvalue_6)
  (bind _returnvalue_7 (UserInterface|CreateWidget "/Game/Blueprints/UI/Actions/WBP_Action_Walk.WBP_Action_Walk_C" _returnvalue))
  (Variables|Default|SetActionWalk _returnvalue_7)
  (bind _returnvalue_8 (UserInterface|CreateWidget "/Game/Blueprints/UI/Actions/WBP_Action_Use.WBP_Action_Use_C" _returnvalue))
  (Variables|Default|SetActionUse _returnvalue_8)
  (bind _returnvalue_9 (UserInterface|CreateWidget "/Game/Blueprints/UI/Actions/WBP_Action_Store.WBP_Action_Store_C" _returnvalue))
  (Variables|Default|SetActionStore _returnvalue_9)
  (bind _returnvalue_10 (UserInterface|CreateWidget "/Game/Blueprints/UI/Actions/WBP_Action_Stop.WBP_Action_Stop_C" _returnvalue))
  (Variables|Default|SetActionStop _returnvalue_10)
  (bind _returnvalue_11 (UserInterface|CreateWidget "/Game/Blueprints/UI/Actions/WBP_Action_Eat.WBP_Action_Eat_C" _returnvalue))
  (Variables|Default|SetActionEat _returnvalue_11)
  (bind _returnvalue_12 (UserInterface|CreateWidget "/Game/Blueprints/UI/Actions/WBP_Action_Repair.WBP_Action_Repair_C" _returnvalue))
  (Variables|Default|SetActionRepair _returnvalue_12))

(fn AddActionCommand
  (params (Selection :type ETTAction%20Enum :default "Walk"))
  (bind _actionrepair (Variables|Default|GetActionRepair))
  (bind _wbp_hudv03 (Variables|Default|GetWBP_HUDv03))
  (bind _actioneat (Variables|Default|GetActionEat))
  (bind _actioncollect (Variables|Default|GetActionCollect))
  (bind _actioncraft (Variables|Default|GetActionCraft))
  (bind _actiondrop (Variables|Default|GetActionDrop))
  (bind _actionequip (Variables|Default|GetActionEquip))
  (bind _actionpickup (Variables|Default|GetActionPickUp))
  (bind _actionuse (Variables|Default|GetActionUse))
  (bind _verticalbox_2 (Variables|/Game/Blueprints/UI/WBP_BasicUI_v03.WBP_BasicUI_v03_C|GetVerticalBox_2 _wbp_hudv03))
  (bind _verticalbox_3 (Variables|/Game/Blueprints/UI/WBP_BasicUI_v03.WBP_BasicUI_v03_C|GetVerticalBox_3 _wbp_hudv03))
  (Widget|Panel|ClearChildren (Variables|/Game/Blueprints/UI/WBP_BasicUI_v03.WBP_BasicUI_v03_C|GetVerticalBox_3 (Variables|Default|GetWBP_HUDv03)))
  (Variables|Default|SetBoxIndex 0)
  (for _array_element (Variables|Default|GetWidgetArray)
    (if (>= (Class|PanelWidget|GetChildrenCount _verticalbox_2) 1)
      (Variables|Default|SetBoxIndex (+ (Variables|Default|GetBoxIndex) 1))
      (if (>= (Class|PanelWidget|GetChildrenCount _verticalbox_3) 3)
        (Variables|Default|SetBoxIndex (+ (Variables|Default|GetBoxIndex) 1))
        (Widget|Panel|AddChild (Variables|/Game/Blueprints/UI/WBP_BasicUI_v03.WBP_BasicUI_v03_C|GetVerticalBox_4 _wbp_hudv03) _array_element)
        (else
          (Widget|Panel|AddChild _verticalbox_3 _array_element)))
      (else
        (Widget|Panel|AddChild _verticalbox_2 _array_element))))
  (switch Utilities|FlowControl|Switch|SwitchonETTAction Selection
    (:Use
      (Widget|Panel|AddChild (CallFunction|GetVerticalBox) _actionuse)
      (Utilities|Array|AddUnique (Variables|Default|GetWidgetArray) _actionuse))
    (:Eat
      (Widget|Panel|AddChild (CallFunction|GetVerticalBox) _actioneat)
      (Utilities|Array|AddUnique (Variables|Default|GetWidgetArray) _actioneat))
    (:PickUp
      (Widget|Panel|AddChild (CallFunction|GetVerticalBox) _actionpickup)
      (Utilities|Array|AddUnique (Variables|Default|GetWidgetArray) _actionpickup))
    (:Drop
      (Widget|Panel|AddChild (CallFunction|GetVerticalBox) _actiondrop)
      (Utilities|Array|AddUnique (Variables|Default|GetWidgetArray) _actiondrop))
    (:Collect
      (Widget|Panel|AddChild (CallFunction|GetVerticalBox) _actioncollect)
      (Utilities|Array|AddUnique (Variables|Default|GetWidgetArray) _actioncollect))
    (:Craft
      (Widget|Panel|AddChild (CallFunction|GetVerticalBox) _actioncraft)
      (Utilities|Array|AddUnique (Variables|Default|GetWidgetArray) _actioncraft))
    (:Repair
      (Widget|Panel|AddChild (CallFunction|GetVerticalBox) _actionrepair)
      (Utilities|Array|AddUnique (Variables|Default|GetWidgetArray) _actionrepair))
    (:Equip
      (Widget|Panel|AddChild (CallFunction|GetVerticalBox) _actionequip)
      (Utilities|Array|AddUnique (Variables|Default|GetWidgetArray) _actionequip))))

(fn RemoveActionCommand
  (params (Selection :type ETTAction%20Enum :default "Walk"))
  (bind _actionrepair (Variables|Default|GetActionRepair))
  (bind _actioneat (Variables|Default|GetActionEat))
  (bind _actioncollect (Variables|Default|GetActionCollect))
  (bind _actioncraft (Variables|Default|GetActionCraft))
  (bind _actiondrop (Variables|Default|GetActionDrop))
  (bind _actionequip (Variables|Default|GetActionEquip))
  (bind _actionpickup (Variables|Default|GetActionPickUp))
  (bind _actionuse (Variables|Default|GetActionUse))
  (switch Utilities|FlowControl|Switch|SwitchonETTAction Selection
    (:Use
      (Widget|RemovefromParent _actionuse)
      (Utilities|Array|RemoveItem (Variables|Default|GetWidgetArray) _actionuse))
    (:Eat
      (Widget|RemovefromParent _actioneat)
      (Utilities|Array|RemoveItem (Variables|Default|GetWidgetArray) _actioneat))
    (:PickUp
      (Widget|RemovefromParent _actionpickup)
      (Utilities|Array|RemoveItem (Variables|Default|GetWidgetArray) _actionpickup))
    (:Drop
      (Widget|RemovefromParent _actiondrop)
      (Utilities|Array|RemoveItem (Variables|Default|GetWidgetArray) _actiondrop))
    (:Collect
      (Widget|RemovefromParent _actioncollect)
      (Utilities|Array|RemoveItem (Variables|Default|GetWidgetArray) _actioncollect))
    (:Craft
      (Widget|RemovefromParent _actioncraft)
      (Utilities|Array|RemoveItem (Variables|Default|GetWidgetArray) _actioncraft))
    (:Repair
      (Widget|RemovefromParent _actionrepair)
      (Utilities|Array|RemoveItem (Variables|Default|GetWidgetArray) _actionrepair))
    (:Equip
      (Widget|RemovefromParent _actionequip)
      (Utilities|Array|RemoveItem (Variables|Default|GetWidgetArray) _actionequip)))
  (CallFunction|ManageVerticalBox))

(fn AddSubTaskTuturial
  (params (Class :type User%20Widget%20Class%20Reference))
  (bind _returnvalue (UserInterface|CreateWidget Class (Game|GetPlayerController 0)))
  (UserInterface|Viewport|AddtoViewport _returnvalue 0))

(fn GetVerticalBox
  (bind _wbp_hudv03 (Variables|Default|GetWBP_HUDv03))
  (return (Utilities|Select :Index (Variables|Default|GetBoxIndex) :Option%200 (Variables|/Game/Blueprints/UI/WBP_BasicUI_v03.WBP_BasicUI_v03_C|GetVerticalBox_2 _wbp_hudv03) :Option%201 (Variables|/Game/Blueprints/UI/WBP_BasicUI_v03.WBP_BasicUI_v03_C|GetVerticalBox_3 _wbp_hudv03) :Option%202 (Variables|/Game/Blueprints/UI/WBP_BasicUI_v03.WBP_BasicUI_v03_C|GetVerticalBox_4 _wbp_hudv03))))

(fn ManageVerticalBox
  (bind _wbp_hudv03 (Variables|Default|GetWBP_HUDv03))
  (bind _verticalbox_2 (Variables|/Game/Blueprints/UI/WBP_BasicUI_v03.WBP_BasicUI_v03_C|GetVerticalBox_2 _wbp_hudv03))
  (bind _verticalbox_3 (Variables|/Game/Blueprints/UI/WBP_BasicUI_v03.WBP_BasicUI_v03_C|GetVerticalBox_3 _wbp_hudv03))
  (Widget|Panel|ClearChildren (Variables|/Game/Blueprints/UI/WBP_BasicUI_v03.WBP_BasicUI_v03_C|GetVerticalBox_3 (Variables|Default|GetWBP_HUDv03)))
  (Variables|Default|SetBoxIndex 0)
  (for _array_element (Variables|Default|GetWidgetArray)
    (if (>= (Class|PanelWidget|GetChildrenCount _verticalbox_2) 1)
      (Variables|Default|SetBoxIndex (+ (Variables|Default|GetBoxIndex) 1))
      (if (>= (Class|PanelWidget|GetChildrenCount _verticalbox_3) 3)
        (Variables|Default|SetBoxIndex (+ (Variables|Default|GetBoxIndex) 1))
        (Widget|Panel|AddChild (Variables|/Game/Blueprints/UI/WBP_BasicUI_v03.WBP_BasicUI_v03_C|GetVerticalBox_4 _wbp_hudv03) _array_element)
        (else
          (Widget|Panel|AddChild _verticalbox_3 _array_element)))
      (else
        (Widget|Panel|AddChild _verticalbox_2 _array_element)))))